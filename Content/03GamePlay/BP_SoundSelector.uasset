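; BP_SoundSelector switches the background music from the stage track to the boss fight track.
; On BeginPlay it spawns the stage BGM cue as a 2D sound once and keeps the reference.
; When any actor begins overlapping its Box, it stops that sound and, after a short delay, spawns the boss BGM cue.
; The overlap has no actor filter or once-only guard, and both events print debug strings.
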(event `self.ReceiveBeginPlay`
  (`KismetSystemLibrary.PrintString` "begi")
  (`/Engine/EditorBlueprintResources/StandardMacros.DoOnce` false
    (:`Completed`
      ;[0 1 0.25] ＢＧＭ再生
      (bind _returnvalue (`GameplayStatics.SpawnSound2D` "/Game/Sounds/BGM/BGM_Stage_Cue.BGM_Stage_Cue" 1.0 1.0 0.0 null))
      (set `self.StageBGM` _returnvalue))))

(event `self.Box.OnComponentBeginOverlap`
  (params (OverlappedComponent :type "PrimitiveComponent Object Reference") (OtherActor :type "Actor Object Reference") (OtherComp :type "PrimitiveComponent Object Reference") (OtherBodyIndex :type Integer) (bFromSweep :type Boolean) (SweepResult :type "HitResult Structure (by ref)"))
  ;[0.4464 0 1] ボス戦
  (`KismetSystemLibrary.PrintString` (`KismetSystemLibrary.GetObjectName` OtherActor))
  (`AudioComponent.Stop` (`self.StageBGM`))
  (`KismetSystemLibrary.Delay` 1.7)
  (`GameplayStatics.SpawnSound2D` "/Game/Sounds/BGM/BGM_Boss_Cue.BGM_Boss_Cue" 1.0 1.0 0.0 null))

(fn `UserConstructionScript`)