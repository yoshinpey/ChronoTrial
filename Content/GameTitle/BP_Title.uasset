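; BP_Title is the title screen controller Blueprint that routes menu input to the title UI widget.
; On BeginPlay, after a short delay, it gets UMGTitle from HUD_Title, focuses it and switches input to Game and UI mode.
; The select up, down and decision input actions call the matching widget functions and print debug strings.
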(event `self.ReceiveBeginPlay`
  ;[0.9622 0.7288 1] 初期化
  (`KismetSystemLibrary.Delay` 0.2)
  (bind _ashud_title (cast `/Game/GameTitle/HUD_Title` (`PlayerController.GetHUD` (`GameplayStatics.GetPlayerController` 0))))
  (bind _output_get (set `self.UMG Title` (`/Game/GameTitle/HUD_Title.UMG_Title` _ashud_title)))
  (`Widget.SetFocus` _output_get)
  (`WidgetBlueprintLibrary.SetInputMode_GameAndUIEx` (`GameplayStatics.GetPlayerController` 0) _output_get))

(event `InputAction|UISelectUp`
  (params (Key :type "Key Structure"))
  ;[0 0.9226 1] UI操作：上がる、下がる、決定
  (:`Pressed`
    (`/Game/GameTitle/UMG_Title.UISelectUp` (`self.UMG Title`))
    (`KismetSystemLibrary.PrintString` "Hello1")))

(event `InputAction|UISelectDown`
  (params (Key :type "Key Structure"))
  ;[0 0.9226 1] UI操作：上がる、下がる、決定
  (:`Pressed`
    (`/Game/GameTitle/UMG_Title.UISelectDown` (`self.UMG Title`))
    (`KismetSystemLibrary.PrintString` "Hello2")))

(event `InputAction|UISelectDecision`
  (params (Key :type "Key Structure"))
  ;[0 0.9226 1] UI操作：上がる、下がる、決定
  (:`Pressed`
    (`/Game/GameTitle/UMG_Title.UISelectDecision` (`self.UMG Title`))
    (`KismetSystemLibrary.PrintString` "Hello3")))

(fn `UserConstructionScript`)