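; CloseDoorBP is a door Blueprint that opens on BeginPlay and exposes a CloseDoor event to shut it again.
; BeginPlay caches the Cube component's relative location, then calls OpenDoor to play a timeline.
; Each timeline update offsets the Cube vertically from that cached position using an ease-out between InitialLocation and NewLocation.
; CloseDoor reverses the same timeline.
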(event `self.ReceiveBeginPlay`
  (set `self.Relative Location` (`SceneComponent.RelativeLocation` (`self.Cube`)))
  (`self.OpenDoor`))

(event `OpenDoor`
  (bind (_relative_location_x _relative_location_y _relative_location_z) (`KismetMathLibrary.BreakVector` (`self.Relative Location`)))
  (bind (_direction `_新規track_0`) (`Timeline|タイムライン_0` :`NewTime` 0.0 :!label _label)
    (:`Update`
      (`SceneComponent.K2_SetRelativeLocation` (`self.Cube`) (`KismetMathLibrary.MakeVector` _relative_location_x _relative_location_y (+ _relative_location_z (`|EaseFunction` "EaseOut" `_新規track_0` (`self.InitialLocation`) (`self.NewLocation`)))) false false))))

(event `CloseDoor`
  (goto _label :!via `Reverse`))

(fn `UserConstructionScript`)