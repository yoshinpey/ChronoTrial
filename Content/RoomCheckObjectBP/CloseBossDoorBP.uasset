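; Boss room door actor built from two cube panels that slide apart and back along their local X axis.
; BeginPlay caches each cube's starting relative location as the base for movement.
; OpenDoor plays a timeline that adds ease-out offsets toward NewLocation for Cube1 and its negation for Cube2.
; CloseDoor reverses the same timeline to bring the panels back.
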(event `self.ReceiveBeginPlay`
  (set `self.Relative Location1` (`SceneComponent.RelativeLocation` (`self.Cube1`)))
  (set `self.Relative Location2` (`SceneComponent.RelativeLocation` (`self.Cube2`))))

(event `OpenDoor`
  (bind (_relative_location2_x _relative_location2_y _relative_location2_z) (`KismetMathLibrary.BreakVector` (`self.Relative Location2`)))
  (bind (_relative_location1_x _relative_location1_y _relative_location1_z) (`KismetMathLibrary.BreakVector` (`self.Relative Location1`)))
  (bind _newlocation (`self.NewLocation`))
  (bind _initiallocation (`self.InitialLocation`))
  (bind (_direction `_新規track_0`) (`Timeline|タイムライン_0` :!label _label)
    (:`Update`
      (`SceneComponent.K2_SetRelativeLocation` (`self.Cube2`) (`KismetMathLibrary.MakeVector` (+ _relative_location2_x (`|EaseFunction` "EaseOut" `_新規track_0` _initiallocation (* _newlocation -1.0))) _relative_location2_y _relative_location2_z) false false)
      (`SceneComponent.K2_SetRelativeLocation` (`self.Cube1`) (`KismetMathLibrary.MakeVector` (+ _relative_location1_x (`|EaseFunction` "EaseOut" `_新規track_0` _initiallocation _newlocation)) _relative_location1_y _relative_location1_z) false false))))

(event `CloseDoor`
  (goto _label :!via `Reverse`))

(fn `UserConstructionScript`)