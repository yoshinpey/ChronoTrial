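; BP_Title controls the title screen, handling menu input and playing an attract movie when left idle.
; On BeginPlay it caches HUD_Title and its widgets, then routes up, down and decision inputs to the title or mode-select widget based on TitleMode.
; In title mode, Tick counts idle time, reset by horizontal mouse movement or key presses.
; Paired DoOnce gates make the HUD start and stop the movie once per transition.
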(event `self.ReceiveBeginPlay`
  ;[1 0.4318 0.8256] 初期化
  (`KismetSystemLibrary.Delay` 0.2)
  (bind _ashud_title (cast `/Game/01GameTitle/HUD_Title` (`PlayerController.GetHUD` (`GameplayStatics.GetPlayerController` 0))))
  (bind _output_get (set `self.As HUD Title` _ashud_title))
  (set `self.UMG Mode Select` (`/Game/01GameTitle/HUD_Title.UMG_ModeSelect` _output_get))
  (set `self.UMG Title Movie` (`/Game/01GameTitle/HUD_Title.UMG_TitleMovie` (`self.As HUD Title`)))
  (set `self.UMG Title` (`/Game/01GameTitle/HUD_Title.UMG_Title` (`self.As HUD Title`)))
  (set `PlayerController.bShowMouseCursor` true (`GameplayStatics.GetPlayerController` 0)))

(event `self.ReceiveTick`
  (params (DeltaSeconds :type "Float (single-precision)"))
  (bind _locationx (`PlayerController.GetMousePosition` (`GameplayStatics.GetPlayerController` 0)))
  (set `self.Delta Seconds` DeltaSeconds)
  (if (`self.TitleMode`)
    (`|ExecutionSequence`
      (:`then_0`
        (if (< (`self.WaitingTimer`) (`self.MaxWaitTime`))
          ;[1 0 0.7345] 放置大麻加算
          (set `self.WaitingTimer` (+ (`self.Delta Seconds`) (`self.WaitingTimer`)))
          (`/Engine/EditorBlueprintResources/StandardMacros.DoOnce` false :!label _label
            (:`Completed`
              (`|ExecutionSequence`
                (:`then_0`
                  ;[1 0 0.0532] 入力によるリセットがかかったら、動画を停止（削除）する
                  (`/Engine/EditorBlueprintResources/StandardMacros.IsValid` (`self.As HUD Title`)
                    (:`Is Valid`
                      (`/Game/01GameTitle/HUD_Title.MovieStop` (`self.As HUD Title`)))))
                (:`then_1`
                  (goto _label_2 :!via `Reset`)))))
          (else
            ;[0 0.9729 1] 大麻が最大になったらPV再生
            (`/Engine/EditorBlueprintResources/StandardMacros.DoOnce` false :!label _label_2
              (:`Completed`
                (`/Engine/EditorBlueprintResources/StandardMacros.IsValid` (`self.As HUD Title`)
                  (:`Is Valid`
                    (`/Game/01GameTitle/HUD_Title.MoviePlay` (`self.As HUD Title`))
                    (goto _label :!via `Reset`))))))))
      (:`then_1`
        ;[0.02797 0.6885 0.08835] マウスが動いたら放置大麻リセット
        (if (!= (`KismetMathLibrary.Abs` (- (`self.preX`) _locationx)) 0.0)
          (set `self.preX` _locationx)
          (set `self.WaitingTimer` 0.0)))
      (:`then_2`
        ;[0.05122 1 0.4711] ボタン押したら大麻リセット
        (if (`self.IsPressed`)
          (set `self.WaitingTimer` 0.0))))))

(event `InputAction|UISelectUp`
  (params (Key :type "Key Structure"))
  (bind _umg_title (`self.UMG Title`))
  (bind _umg_mode_select (`self.UMG Mode Select`))
  ;[0 0.9226 1] UI操作：上がる、下がる、決定
  (:`Pressed`
    (if (`self.TitleMode`) :!label _label_3
      (`/Engine/EditorBlueprintResources/StandardMacros.IsValid` _umg_title
        (:`Is Valid`
          (`/Game/01GameTitle/UMG_Title.UISelectUp` _umg_title)))
      (else
        (`/Engine/EditorBlueprintResources/StandardMacros.IsValid` _umg_mode_select
          (:`Is Valid`
            (`/Game/02GameSelect/UMG_ModeSelect.UISelectUp` _umg_mode_select)))))))

(event `Key|Gamepad_LeftStick_Up`
  (params (Key :type "Key Structure"))
  ;[0 0.9226 1] UI操作：上がる、下がる、決定
  (:`Pressed`
    (goto _label_3)))

(event `InputAction|UISelectDown` :paused true
  (params (Key :type "Key Structure"))
  (bind _umg_title (`self.UMG Title`))
  (bind _umg_mode_select (`self.UMG Mode Select`))
  ;[0 0.9226 1] UI操作：上がる、下がる、決定
  (:`Pressed`
    (if (`self.TitleMode`) :!label _label_4
      (`/Engine/EditorBlueprintResources/StandardMacros.IsValid` _umg_title
        (:`Is Valid`
          (`/Game/01GameTitle/UMG_Title.UISelectDown` _umg_title)))
      (else
        (`/Engine/EditorBlueprintResources/StandardMacros.IsValid` _umg_mode_select
          (:`Is Valid`
            (`/Game/02GameSelect/UMG_ModeSelect.UISelectDown` _umg_mode_select)))))))

(event `Key|Gamepad_LeftStick_Down` :paused true
  (params (Key :type "Key Structure"))
  ;[0 0.9226 1] UI操作：上がる、下がる、決定
  (:`Pressed`
    (goto _label_4)))

(event `InputAction|UISelectDecision`
  (params (Key :type "Key Structure"))
  (bind _umg_mode_select (`self.UMG Mode Select`))
  (bind _umg_title (`self.UMG Title`))
  ;[0 0.9226 1] UI操作：上がる、下がる、決定
  (:`Pressed`
    (if (`self.TitleMode`)
      (`/Engine/EditorBlueprintResources/StandardMacros.IsValid` _umg_title
        (:`Is Valid`
          (`/Game/01GameTitle/UMG_Title.UISelectDecision` _umg_title)))
      (else
        (`/Engine/EditorBlueprintResources/StandardMacros.IsValid` _umg_mode_select
          (:`Is Valid`
            (`/Game/02GameSelect/UMG_ModeSelect.UISelectDecision` _umg_mode_select)))))))

(event `Key|AnyKey`
  (params (Key :type "Key Structure"))
  ;[0.4189 0.4016 1] 何らかのキー入力があったらリセットフラグ入れる
  (:`Pressed`
    (if (`self.TitleMode`)
      (set `self.IsPressed` true)
      (`KismetSystemLibrary.Delay` (`self.Delta Seconds`))
      (set `self.IsPressed` false))))

(fn `UserConstructionScript`)