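; Base enemy projectile that damages the player and supports the time-stop and rewind skills.
; Capsule overlaps route by tag: during time stop, player bullets or sword deflect it away from the player, letting it damage enemies and trigger the HUD hit mark.
; On hit it freezes and hides for a GameInstance-set countdown before destruction.
; Tick resurrects it if rewinding restores that countdown, and slows deflected bullets during player deceleration.
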(event `self.ReceiveBeginPlay`
  (bind _asmy_game_instance (cast `MyGameInstance` (`GameplayStatics.GetGameInstance`))
    (:`then`
      (bind _output_get (set `self.DeathWaitTime` (`KismetMathLibrary.Conv_IntToDouble` (`MyGameInstance.ReverseTime` _asmy_game_instance))))
      (set `self.DeathTime` _output_get)
      (set `self.ReverseSpeed` (`MyGameInstance.ReverseSpeed` _asmy_game_instance))
      (set `self.MaxSpeed` (`ProjectileMovementComponent.MaxSpeed` (`self.ProjectileMovement`)))
      (bind _asthird_person_character (cast `/Game/ThirdPersonBP/Blueprints/ThirdPersonCharacter` (`GameplayStatics.GetPlayerPawn` 0)))
      (set `self.Player Skill Manager` (`/Game/ThirdPersonBP/Blueprints/ThirdPersonCharacter.PlayerSkillManager` _asthird_person_character)))
    (:`CastFailed`
      (`KismetSystemLibrary.PrintString` "BulletBase_Cast"))))

(event `self.Capsule.OnComponentBeginOverlap`
  (params (OverlappedComponent :type "PrimitiveComponent Object Reference") (OtherActor :type "Actor Object Reference") (OtherComp :type "PrimitiveComponent Object Reference") (OtherBodyIndex :type Integer) (bFromSweep :type Boolean) (SweepResult :type "HitResult Structure (by ref)"))
  ;[1 0.2448 0.7127] Hit / Overlap
  (`/Engine/EditorBlueprintResources/StandardMacros.IsValid` OtherComp
    (:`Is Valid`
      (`|ExecutionSequence`
        (:`then_0`
          (for _array_element (`Actor.Tags` OtherActor)
            (switch `name` _array_element
              (:`Player`
                (`self.PlayerHit` OtherActor)
                (break))
              (:`PlayerBullet`
                (`self.PlayerAttackHit` OtherActor)
                (break))
              (:`Enemy`
                (`self.EnemyHit` OtherActor)
                (break)))))
        (:`then_1`
          (if (`ActorComponent.ComponentHasTag` OtherComp "PlayerSword")
            (`self.PlayerAttackHit` OtherActor)))))))

(event `self.ReceiveHit`
  (params (MyComp :type "PrimitiveComponent Object Reference") (Other :type "Actor Object Reference") (OtherComp :type "PrimitiveComponent Object Reference") (bSelfMoved :type Boolean) (HitLocation :type "Vector Structure") (HitNormal :type "Vector Structure") (NormalImpulse :type "Vector Structure") (Hit :type "HitResult Structure (by ref)"))
  ;[1 0.2448 0.7127] Hit / Overlap
  (`self.BulletHit`)
  (`GameplayStatics.SpawnEmitterAtLocation` "/Game/StarterContent/Particles/P_Explosion.P_Explosion" (`self.K2_GetActorLocation` self)))

(event `self.ReceiveTick`
  (params (DeltaSeconds :type "Float (single-precision)"))
  (bind _capsule (`self.Capsule`))
  (`|ExecutionSequence`
    (:`then_0`
      ;[0.5341 0.4595 1] 減速中のスピード変化
      (if (`self.Reflection`)
        (set `ProjectileMovementComponent.MaxSpeed` (`KismetMathLibrary.SelectFloat` (* (`self.MaxSpeed`) (`/Game/ThirdPersonBP/Blueprints/Skill/PlayerSkillManager.DecelSpeed` (`self.Player Skill Manager`))) (`self.MaxSpeed`) (`/Game/ThirdPersonBP/Blueprints/Skill/PlayerSkillManager.IsDecel` (`self.Player Skill Manager`))) (`self.ProjectileMovement`))))
    (:`then_1`
      (if (`self.IsHit`)
        (if (`/Game/Reverse/UReverseTimeComponent.Reversing` (`self.UEnemyBulletReverseTime`))
          ;[0.2156 1 0.2429] 生き返り
          (set `self.DeathTime` (+ (`self.DeathTime`) (`self.ReverseSpeed`)))
          (if (>= (`self.DeathTime`) (`self.DeathWaitTime`))
            (`self.Resurrection`))
          (else
            ;[1 0.9519 0.4514] 通常処理（消すやつ
            (`/Engine/EditorBlueprintResources/StandardMacros.DecrementFloat` (`self.DeathTime`)
              (:`  `
                (if (<= (`self.DeathTime`) 0.0)
                  ;;[1 0.0221 0] 削除
                  (`ActorComponent.K2_DestroyComponent` (`self.UEnemyBulletReverseTime`))
                  (`self.K2_DestroyActor`)
                  (elif (`self.FirstDeathSwitch`)
                    (set `self.FirstDeathSwitch` false)
                    (`ActorComponent.SetComponentTickEnabled` (`self.UEnemyBulletReverseTime`) false)
                    (`KismetSystemLibrary.PrintString` "Hello")))))))
        (else
          (set `self.FirstDeathSwitch` true))))
    (:`then_2`
      (if (`KismetSystemLibrary.IsValid` (`self.UEnemyBulletReverseTime`))
        (if (or (`/Game/Reverse/UReverseTimeComponent.Reversing` (`self.UEnemyBulletReverseTime`)) (`self.IsHit`))
          (`PrimitiveComponent.SetCollisionEnabled` _capsule "NoCollision")
          (else
            (`PrimitiveComponent.SetCollisionEnabled` _capsule "QueryAndPhysics")))))))

(event `StopDangan`
  ;[1 1 1] Stop
  (set `self.HitVelocity` (`MovementComponent.Velocity` (`self.ProjectileMovement`)))
  (set `ProjectileMovementComponent.MaxSpeed` 0.0001 (`self.ProjectileMovement`)))

(event `RestartDangan`
  ;[1 1 1] Stop
  (set `ProjectileMovementComponent.MaxSpeed` (`self.MaxSpeed`) (`self.ProjectileMovement`))
  (`ProjectileMovementComponent.SetVelocityInLocalSpace` (`self.ProjectileMovement`) (`KismetMathLibrary.MakeVector` (`self.MaxSpeed`))))

(fn `BulletHit`
  (set `self.IsHit` true)
  (set `self.IsDead` true)
  (`self.StopDangan`)
  (`self.SetActorHiddenInGame` true))

(fn `EnemyHit`
  (params (HitActor :type "Actor Object Reference"))
  (if (`self.Reflection`)
    (bind _asthird_person_character (cast `/Game/ThirdPersonBP/Blueprints/ThirdPersonCharacter` (`GameplayStatics.GetPlayerPawn` 0)))
    (if (`/Game/ThirdPersonBP/Blueprints/Skill/PlayerSkillManager.IsStop` (`/Game/ThirdPersonBP/Blueprints/ThirdPersonCharacter.PlayerSkillManager` _asthird_person_character))
      (`GameplayStatics.ApplyDamage` HitActor (`self.Base Damage`) null self)
      (`GameplayStatics.SpawnEmitterAtLocation` "/Game/StarterContent/Particles/P_Explosion.P_Explosion" (`self.K2_GetActorLocation` self))
      (`self.BulletHit`)
      ;[1 0.2843 0.6635] HitMark
      (bind _ashud_play (cast `/Game/GamePlay/HUD_Play` (`PlayerController.GetHUD` (`GameplayStatics.GetPlayerController` 0)))
        (:`then`
          (`/Game/ThirdPersonBP/Blueprints/Gun/UI/WG_HitMark.AttackHit` (`/Game/GamePlay/HUD_Play.HitMarkWidget` _ashud_play)))
        (:`CastFailed`
          (`KismetSystemLibrary.PrintString` "EnemyBulletBase_Cast"))))))

(fn `PlayerAttackHit`
  (params (HitActor :type "Actor Object Reference"))
  (bind _asthird_person_character (cast `/Game/ThirdPersonBP/Blueprints/ThirdPersonCharacter` (`GameplayStatics.GetPlayerPawn` 0)))
  (if (`/Game/ThirdPersonBP/Blueprints/Skill/PlayerSkillManager.IsStop` (`/Game/ThirdPersonBP/Blueprints/ThirdPersonCharacter.PlayerSkillManager` _asthird_person_character))
    (if (`self.Reflection`)
      _
      (elif (not (`self.IsHit`))
        (set `ProjectileMovementComponent.MaxSpeed` (`self.MaxSpeed`) (`self.ProjectileMovement`))
        (`self.SetActorTickEnabled` self true)
        (set `self.CustomTimeDilation` 1.0)
        (`PrimitiveComponent.SetCollisionEnabled` (`self.Capsule`) "QueryAndPhysics")
        (bind _output_get (set `self.HitVelocity` (* (`KismetMathLibrary.Normal` (- (`self.K2_GetActorLocation`) (`self.K2_GetActorLocation` (`GameplayStatics.GetPlayerPawn` 0)))) (`ProjectileMovementComponent.MaxSpeed` (`self.ProjectileMovement`)))))
        (set `MovementComponent.Velocity` _output_get (`self.ProjectileMovement`))
        (`GameplayStatics.SpawnEmitterAtLocation` "/Game/StarterContent/Particles/P_Explosion.P_Explosion" (`self.K2_GetActorLocation` self) (struct) (0.3 0.3 0.3))
        (set `self.Reflection` true)
        (bind _asbp_player_bullet (cast `/Game/ThirdPersonBP/Blueprints/Gun/BP_PlayerBullet` HitActor)
          (:`then`
            (set `/Game/ThirdPersonBP/Blueprints/Gun/BP_PlayerBullet.IsHit` true _asbp_player_bullet)
            (`/Game/ThirdPersonBP/Blueprints/Gun/BP_PlayerBullet.StopDangan` _asbp_player_bullet)
            (`self.SetActorHiddenInGame` _asbp_player_bullet true)
            (`PrimitiveComponent.SetCollisionEnabled` (`/Game/ThirdPersonBP/Blueprints/Gun/BP_PlayerBullet.Capsule` _asbp_player_bullet) "NoCollision"))
          (:`CastFailed`
            (`KismetSystemLibrary.PrintString` "EnemyBullet_Cast")))))))

(fn `PlayerHit`
  (params (HitActor :type "Actor Object Reference"))
  (if (`self.IsHit`)
    (`KismetSystemLibrary.PrintString` "IsHited")
    (elif (`self.Reflection`)
      (`KismetSystemLibrary.PrintString` "IsReflect")
      (else
        (bind _asthird_person_character (cast `/Game/ThirdPersonBP/Blueprints/ThirdPersonCharacter` (`GameplayStatics.GetPlayerPawn` 0)))
        (if (not (`/Game/ThirdPersonBP/Blueprints/Skill/PlayerSkillManager.IsStop` (`/Game/ThirdPersonBP/Blueprints/ThirdPersonCharacter.PlayerSkillManager` _asthird_person_character)))
          (`GameplayStatics.ApplyDamage` HitActor (`self.Base Damage`) null self)
          (`GameplayStatics.SpawnEmitterAtLocation` "/Game/StarterContent/Particles/P_Explosion.P_Explosion" (`self.K2_GetActorLocation` self))
          (`self.BulletHit`))))))

(fn `Resurrection`
  (set `self.DeathTime` (`self.DeathWaitTime`))
  (`self.SetActorHiddenInGame` false)
  (set `self.IsHit` false)
  (set `self.IsDead` false)
  (`ActorComponent.SetComponentTickEnabled` (`self.UEnemyBulletReverseTime`) true)
  (`self.RestartDangan`))

(fn `SetDefaultCollisionPriset`
  (`PrimitiveComponent.SetCollisionResponseToChannel` (`self.Capsule`) "ECC_GameTraceChannel3" "ECR_Overlap"))

(fn `UserConstructionScript`)