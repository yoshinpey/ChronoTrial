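; Test bullet actor that damages actors tagged Enemy and explodes when it overlaps something.
; On BeginPlay it applies a fixed 90-degree rotation offset relative to its current orientation.
; Overlaps with ThirdPersonCharacter and other BP_BulletTest instances are ignored.
; Any other overlap prints the actor's name, spawns a scaled-down explosion and destroys the bullet, first applying damage and enabling a particle emitter for enemies.
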(event `self.ReceiveBeginPlay`
  (`self.K2_SetActorRotation` (`KismetMathLibrary.TransformRotation` (`KismetMathLibrary.MakeTransform` (0.0 0.0 0.0) (`self.K2_GetActorRotation`)) (struct :`Pitch` -90.0))))

(event `self.ReceiveActorBeginOverlap`
  (params (OtherActor :type "Actor Object Reference"))
  (bind _returnvalue (`GameplayStatics.GetObjectClass` OtherActor))
  (`/Engine/EditorBlueprintResources/StandardMacros.IsValid` OtherActor
    (:`Is Valid`
      (if (not (or (== _returnvalue "/Game/ThirdPersonBP/Blueprints/ThirdPersonCharacter.ThirdPersonCharacter_C") (== _returnvalue "BP_BulletTest_C")))
        (`|ExecutionSequence`
          (:`then_0`
            (if (`self.ActorHasTag` OtherActor "Enemy")
              (`GameplayStatics.ApplyDamage` OtherActor 1.0 null self)
              (`FXSystemComponent.SetEmitterEnable` (`self.ParticleSystem`) "None" true)))
          (:`then_1`
            (`KismetSystemLibrary.PrintString` (`KismetSystemLibrary.GetDisplayName` OtherActor))
            (`GameplayStatics.SpawnEmitterAtLocation` "/Game/StarterContent/Particles/P_Explosion.P_Explosion" (`self.K2_GetActorLocation` self) (struct) (* (`self.GetActorScale3D` self) 0.2))
            (`self.K2_DestroyActor` self)))))))

(fn `UserConstructionScript`)