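; BP_TestEnemy is a test melee enemy character that damages the player and explodes when its health runs out.
; AttackEvent stores the damage amount and toggles the right attack collider, whose overlap applies that damage to the player character only.
; AnyDamage reduces Health; at zero it disables capsule collision, detaches the controller, plays an animation and explosion, then explodes again after a delay and destroys itself.
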(event `self.ReceiveBeginPlay`
  (`PrimitiveComponent.SetCollisionEnabled` (`self.RightAttackCollider`) "NoCollision"))

(event `self.ReceiveAnyDamage`
  (params (Damage :type "Float (single-precision)") (DamageType :type "DamageType Object Reference") (InstigatedBy :type "Controller Object Reference") (DamageCauser :type "Actor Object Reference"))
  (bind _output_get (set `self.Health` (- (`self.Health`) Damage)))
  (if (<= _output_get 0.0)
    (`PrimitiveComponent.SetCollisionEnabled` (`self.CapsuleComponent`) "NoCollision")
    (`self.DetachFromControllerPendingDestroy`)
    (`SkeletalMeshComponent.PlayAnimation` (`self.Mesh`) "/Game/Enemy/Anim/TestEnemy_Jump_Loop.TestEnemy_Jump_Loop" false)
    (`GameplayStatics.SpawnEmitterAtLocation` "/Game/StarterContent/Particles/P_Explosion.P_Explosion" (`self.K2_GetActorLocation`))
    (`KismetSystemLibrary.Delay` 3.0)
    (`GameplayStatics.SpawnEmitterAtLocation` "/Game/StarterContent/Particles/P_Explosion.P_Explosion" (`self.K2_GetActorLocation`))
    (`self.K2_DestroyActor`)))

(event `/Game/Enemy/Character_Interface.AttackEvent`
  (params (Damage :type "Float (single-precision)") (IsBegin :type Boolean))
  (set `self.Damage` Damage)
  (if IsBegin
    (`PrimitiveComponent.SetCollisionEnabled` (`self.RightAttackCollider`) "QueryAndPhysics")
    (else
      (`PrimitiveComponent.SetCollisionEnabled` (`self.RightAttackCollider`) "NoCollision"))))

(event `self.RightAttackCollider.OnComponentBeginOverlap`
  (params (OverlappedComponent :type "PrimitiveComponent Object Reference") (OtherActor :type "Actor Object Reference") (OtherComp :type "PrimitiveComponent Object Reference") (OtherBodyIndex :type Integer) (bFromSweep :type Boolean) (SweepResult :type "HitResult Structure (by ref)"))
  (bind _returnvalue (`GameplayStatics.GetPlayerCharacter` 0))
  (if (== OtherActor _returnvalue)
    (`GameplayStatics.ApplyDamage` _returnvalue (`self.Damage`))))

(fn `UserConstructionScript`)