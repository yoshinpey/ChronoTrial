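; Test enemy bullet that damages the player and leaves marks on surfaces it hits, extending a parent that owns BeginPlay and Tick logic.
; A blocking hit spawns a temporary bullet-mark decal aligned to the impact normal.
; Overlapping an actor tagged Player applies damage and spawns an explosion.
; Both paths flag the hit, call StopDangan, hide the bullet and disable capsule collision, without destroying it here.
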(event `self.ReceiveBeginPlay`
  (`parent.ReceiveBeginPlay`))

(event `self.ReceiveTick`
  (params (DeltaSeconds :type "Float (single-precision)"))
  (`parent.ReceiveTick` DeltaSeconds))

(event `self.ReceiveHit`
  (params (MyComp :type "PrimitiveComponent Object Reference") (Other :type "Actor Object Reference") (OtherComp :type "PrimitiveComponent Object Reference") (bSelfMoved :type Boolean) (HitLocation :type "Vector Structure") (HitNormal :type "Vector Structure") (NormalImpulse :type "Vector Structure") (Hit :type "HitResult Structure (by ref)"))
  (`GameplayStatics.SpawnDecalAtLocation` "/Game/ThirdPersonBP/BulletMark_Mat1.BulletMark_Mat1" (10.0 10.0 10.0) HitLocation (`KismetMathLibrary.Conv_VectorToRotator` HitNormal) 10.0)
  (set `self.IsHit` true)
  (`self.StopDangan`)
  (`self.SetActorHiddenInGame` true)
  (`PrimitiveComponent.SetCollisionEnabled` (`self.Capsule`) "NoCollision"))

(event `self.ReceiveActorBeginOverlap`
  (params (OtherActor :type "Actor Object Reference"))
  (`/Engine/EditorBlueprintResources/StandardMacros.IsValid` OtherActor
    (:`Is Valid`
      (if (`self.ActorHasTag` OtherActor "Player")
        (`GameplayStatics.ApplyDamage` OtherActor (`self.Base Damage`) null self)
        (`FXSystemComponent.SetEmitterEnable` (`self.ParticleSystem`) "None" true)
        (`GameplayStatics.SpawnEmitterAtLocation` "/Game/StarterContent/Particles/P_Explosion.P_Explosion" (`self.K2_GetActorLocation` self))
        (set `self.IsHit` true)
        (`self.StopDangan`)
        (`self.SetActorHiddenInGame` true)
        (`PrimitiveComponent.SetCollisionEnabled` (`self.Capsule`) "NoCollision")))))

(fn `UserConstructionScript`)