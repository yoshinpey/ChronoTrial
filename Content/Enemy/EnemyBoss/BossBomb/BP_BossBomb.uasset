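; BP_BossBomb is a boss bomb that shows a telegraphed blast area, then explodes after a timed delay.
; BeginPlay sizes the outline ring through material scalars, and Tick grows an inner indicator's radius as the fuse elapses.
; On expiry it spawns an explosion emitter and briefly enables sphere collision, which damages the first overlapping actor and switches off.
; The indicators then hide, and the actor destroys itself when its kill timer runs out.
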(event `self.ReceiveBeginPlay`
  (bind _outlinestaticmesh (`self.OutLineStaticMesh`))
  ;[1 1 1] Out
  (`MeshComponent.SetScalarParameterValueOnMaterials` _outlinestaticmesh "Outer" (`self.MaxSize`))
  (`MeshComponent.SetScalarParameterValueOnMaterials` _outlinestaticmesh "Inner" (- (`self.MaxSize`) (`self.OutLineSize`)))
  ;[1 1 1] Current
  (`MeshComponent.SetScalarParameterValueOnMaterials` (`self.CurrentStaticMesh`) "Outer" (`self.MaxSize`)))

(event `self.ReceiveTick`
  (params (DeltaSeconds :type "Float (single-precision)"))
  (set `self.LifeTime` (+ (`self.LifeTime`) DeltaSeconds))
  (if (`self.IsExplod`)
    (set `self.KillTime` (- (`self.KillTime`) DeltaSeconds))
    (bind _output_get (set `self.CollidValidTime` (- (`self.CollidValidTime`) DeltaSeconds)))
    (if (< _output_get 0.0)
      (`PrimitiveComponent.SetCollisionEnabled` (`self.Sphere`) "NoCollision")
      (`SceneComponent.SetVisibility` (`self.OutLineStaticMesh`) false false)
      (`SceneComponent.SetVisibility` (`self.CurrentStaticMesh`) false false))
    (if (<= (`self.KillTime`) 0.0)
      (`self.K2_DestroyActor`))
    (else
      (set `self.CurrentSize` (/ (`self.LifeTime`) (`self.ExplodeWaitTime`)))
      (`MeshComponent.SetScalarParameterValueOnMaterials` (`self.CurrentStaticMesh`) "Outer" (* (`self.CurrentSize`) 0.5))
      (if (>= (`self.LifeTime`) (`self.ExplodeWaitTime`))
        (`GameplayStatics.SpawnEmitterAtLocation` "/Game/StarterContent/Particles/P_Explosion.P_Explosion" (`self.K2_GetActorLocation`) (struct) (`self.ExplodeScale`))
        (set `self.IsExplod` true)
        (`PrimitiveComponent.SetCollisionEnabled` (`self.Sphere`) "QueryOnly")
        (set `self.CollidValidTime` 0.4)))))

(event `self.Sphere.OnComponentBeginOverlap`
  (params (OverlappedComponent :type "PrimitiveComponent Object Reference") (OtherActor :type "Actor Object Reference") (OtherComp :type "PrimitiveComponent Object Reference") (OtherBodyIndex :type Integer) (bFromSweep :type Boolean) (SweepResult :type "HitResult Structure (by ref)"))
  (`GameplayStatics.ApplyDamage` OtherActor 30.0)
  (`PrimitiveComponent.SetCollisionEnabled` (`self.Sphere`) "NoCollision"))

(fn `UserConstructionScript`)