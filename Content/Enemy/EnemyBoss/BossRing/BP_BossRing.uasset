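; BP_BossRing is a timed ring effect for the boss enemy that expands over its lifetime and destroys itself when KillTime runs out.
; Each tick, LifeTime relative to FullWaitTime drives Outer and Inner in the Ring_Out_Data material parameter collection, with Inner trailing by OutLineSize.
; Five OutLine components spin by a fixed step per frame, independent of delta time.
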(event `self.ReceiveBeginPlay`
  ;[1 1 1] Out
  (`KismetMaterialLibrary.SetScalarParameterValue` "/Game/Enemy/EnemyBoss/BossRing/Ring_Out_Data.Ring_Out_Data" "Outer")
  (`KismetMaterialLibrary.SetScalarParameterValue` "/Game/Enemy/EnemyBoss/BossRing/Ring_Out_Data.Ring_Out_Data" "Inner" (`self.OutLineSize`)))

(event `self.ReceiveTick`
  (params (DeltaSeconds :type "Float (single-precision)"))
  (bind _returnvalue (* (/ (`self.LifeTime`) (`self.FullWaitTime`)) 0.5))
  (set `self.LifeTime` (+ (`self.LifeTime`) DeltaSeconds))
  (set `self.KillTime` (- (`self.KillTime`) DeltaSeconds))
  (if (<= (`self.KillTime`) 0.0)
    (`self.K2_DestroyActor`)
    (else
      (`KismetMaterialLibrary.SetScalarParameterValue` "/Game/Enemy/EnemyBoss/BossRing/Ring_Out_Data.Ring_Out_Data" "Outer" _returnvalue)
      (`KismetMaterialLibrary.SetScalarParameterValue` "/Game/Enemy/EnemyBoss/BossRing/Ring_Out_Data.Ring_Out_Data" "Inner" (- _returnvalue (`self.OutLineSize`)))
      (for _array_element (`|MakeArray` (`self.OutLine1`) (`self.OutLine2`) (`self.OutLine3`) (`self.OutLine4`) (`self.OutLine5`))
        (`SceneComponent.K2_AddWorldRotation` _array_element (struct :`Yaw` 5.0) false false)))))

(fn `UserConstructionScript`)