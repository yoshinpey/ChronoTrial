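; BP_Explode appears to be a boss explosion indicator that animates a ring-shaped visual through two Material Parameter Collections.
; BeginPlay sets the fixed outline's outer and inner bounds from MaxSize and OutLineSize, plus the current ring's outer bound.
; Tick drives the current ring's inner bound from elapsed time over MaxWaitTime, unclamped, and prints it for debugging.
; No damage, detonation or cleanup logic is present.
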(event `self.ReceiveBeginPlay`
  ;[1 1 1] Out
  (`KismetMaterialLibrary.SetScalarParameterValue` "/Game/Enemy/EnemyBoss/Explode_Out_Data.Explode_Out_Data" "Outer" (`self.MaxSize`))
  (`KismetMaterialLibrary.SetScalarParameterValue` "/Game/Enemy/EnemyBoss/Explode_Out_Data.Explode_Out_Data" "Inner" (- (`self.MaxSize`) (`self.OutLineSize`)))
  (`KismetMaterialLibrary.SetScalarParameterValue` "/Game/Enemy/EnemyBoss/Explode_Current_Data.Explode_Current_Data" "Outer" (`self.MaxSize`)))

(event `self.ReceiveTick`
  (params (DeltaSeconds :type "Float (single-precision)"))
  (set `self.LifeTime` (+ (`self.LifeTime`) DeltaSeconds))
  (set `self.CurrentSize` (/ (`self.LifeTime`) (`self.MaxWaitTime`)))
  (`KismetMaterialLibrary.SetScalarParameterValue` "/Game/Enemy/EnemyBoss/Explode_Current_Data.Explode_Current_Data" "Inner" (- (`self.CurrentSize`) (`self.OutLineSize`)))
  (`KismetSystemLibrary.PrintString` (`KismetStringLibrary.Conv_DoubleToString` (`self.CurrentSize`)) true true (struct :`G` 0.66 :`B` 1.0 :`A` 1.0) 0.0))

(fn `UserConstructionScript`)