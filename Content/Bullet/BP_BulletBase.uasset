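; Base projectile bullet that damages Enemy-tagged actors on overlap and supports being brought back by time reversal.
; On a hit it leaves a decal or explosion, then stops, hides and counts down to destruction instead of being destroyed immediately.
; Reversing refills that countdown at the GameInstance's reverse speed; once full, the bullet reappears and relaunches.
; Capsule collision stays off while reversing or in the hit state.
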(event `self.ReceiveBeginPlay`
  (bind _asnew_game_instance (cast `/Game/NewGameInstance` (`GameplayStatics.GetGameInstance`)))
  (bind _output_get (set `self.DeathWaitTime` (`KismetMathLibrary.Conv_IntToDouble` (`/Game/NewGameInstance.ReverseTime` _asnew_game_instance))))
  (set `self.DeathTime` _output_get)
  (set `self.ReverseSpeed` (`/Game/NewGameInstance.ReverseSpeed` _asnew_game_instance))
  (set `self.MaxSpeed` (`ProjectileMovementComponent.MaxSpeed` (`self.ProjectileMovement`))))

(event `self.ReceiveTick`
  (params (DeltaSeconds :type "Float (single-precision)"))
  (bind _capsule (`self.Capsule`))
  (`|ExecutionSequence`
    (:`then_0`
      (if (`self.IsHit`)
        (if (`/Game/Reverse/UReverseTimeComponent.Reversing` (`self.UReverseTimeComponent`))
          (set `self.DeathTime` (+ (`self.DeathTime`) (* (`self.ReverseSpeed`) 1.0)))
          ;[1 1 1] 生き返り
          (if (>= (`self.DeathTime`) (`self.DeathWaitTime`))
            (set `self.DeathTime` (`self.DeathWaitTime`))
            (set `self.IsHit` false)
            (`ActorComponent.SetComponentTickEnabled` (`self.UReverseTimeComponent`) true)
            (`self.RestartDangan`)
            (`self.SetActorHiddenInGame` false))
          (else
            (`/Engine/EditorBlueprintResources/StandardMacros.DecrementFloat` (`self.DeathTime`)
              (:`  `
                (if (<= (`self.DeathTime`) 0.0)
                  (`ActorComponent.K2_DestroyComponent` (`self.UReverseTimeComponent`))
                  (`self.K2_DestroyActor`)
                  (elif (`self.FirstDeathSwitch`)
                    (set `self.FirstDeathSwitch` false)
                    (`ActorComponent.SetComponentTickEnabled` (`self.UReverseTimeComponent`) false)))))))
        (else
          (set `self.FirstDeathSwitch` true))))
    (:`then_1`
      (if (`KismetSystemLibrary.IsValid` (`self.UReverseTimeComponent`))
        (if (or (`/Game/Reverse/UReverseTimeComponent.Reversing` (`self.UReverseTimeComponent`)) (`self.IsHit`))
          (`PrimitiveComponent.SetCollisionEnabled` _capsule "NoCollision")
          (else
            (`PrimitiveComponent.SetCollisionEnabled` _capsule "QueryAndPhysics")))))))

(event `StopDangan`
  ;[1 1 1] Stop
  (set `ProjectileMovementComponent.MaxSpeed` 0.0001 (`self.ProjectileMovement`)))

(event `self.ReceiveHit`
  (params (MyComp :type "PrimitiveComponent Object Reference") (Other :type "Actor Object Reference") (OtherComp :type "PrimitiveComponent Object Reference") (bSelfMoved :type Boolean) (HitLocation :type "Vector Structure") (HitNormal :type "Vector Structure") (NormalImpulse :type "Vector Structure") (Hit :type "HitResult Structure (by ref)"))
  (bind _returnvalue (`GameplayStatics.SpawnDecalAtLocation` "/Game/ThirdPersonBP/BulletMark_Mat1.BulletMark_Mat1" (10.0 10.0 10.0) HitLocation (`KismetMathLibrary.Conv_VectorToRotator` HitNormal) 10.0))
  (`DecalComponent.SetFadeScreenSize` _returnvalue 0.01)
  (set `self.IsHit` true)
  (`self.StopDangan`)
  (`self.SetActorHiddenInGame` true)
  (`PrimitiveComponent.SetCollisionEnabled` (`self.Capsule`) "NoCollision"))

(event `RestartDangan`
  (bind _projectilemovement (`self.ProjectileMovement`))
  ;[1 1 1] Stop
  (set `ProjectileMovementComponent.MaxSpeed` (`self.MaxSpeed`) _projectilemovement)
  (`ProjectileMovementComponent.SetVelocityInLocalSpace` _projectilemovement (`KismetMathLibrary.MakeVector` (`self.MaxSpeed`))))

(event `self.ReceiveActorBeginOverlap`
  (params (OtherActor :type "Actor Object Reference"))
  (`/Engine/EditorBlueprintResources/StandardMacros.IsValid` OtherActor
    (:`Is Valid`
      (if (`self.ActorHasTag` OtherActor "Enemy")
        (`GameplayStatics.ApplyDamage` OtherActor (`self.Base Damage`) null self)
        (`GameplayStatics.SpawnEmitterAtLocation` "/Game/StarterContent/Particles/P_Explosion.P_Explosion" (`self.K2_GetActorLocation` self))
        (set `self.IsHit` true)
        (`self.StopDangan`)
        (`self.SetActorHiddenInGame` true)
        (`PrimitiveComponent.SetCollisionEnabled` (`self.Capsule`) "NoCollision")))))

(fn `UserConstructionScript`)