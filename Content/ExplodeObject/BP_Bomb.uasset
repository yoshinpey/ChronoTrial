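; Time-rewindable bomb actor that spins idle until hit by sword or bullet, then flies away from the player, smokes and explodes.
; Tick runs waiting, fuse, explode and end phases using bool flags and a shared timer.
; The blast enlarges the overlap sphere, damaging each Player or Enemy once.
; UReverseTimeComponent switches to reverse phase handlers, and destruction waits out the GameInstance rewind window so explosions can be undone.
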(event `self.ReceiveBeginPlay`
  ;[1 1 1] 初期化
  (bind _asthird_person_character (cast `/Game/ThirdPersonBP/Blueprints/ThirdPersonCharacter` (`GameplayStatics.GetPlayerPawn` 0)))
  (set `self.As Third Person Character` _asthird_person_character)
  (bind _asmy_game_instance (cast `MyGameInstance` (`GameplayStatics.GetGameInstance`)))
  (set `self.As My Game Instance` _asmy_game_instance)
  (bind _asmy_game_instance_2 (cast `MyGameInstance` (`GameplayStatics.GetGameInstance`)))
  (set `self.DeathWaitTime` (/ (`KismetMathLibrary.Conv_IntToDouble` (`MyGameInstance.ReverseTime` _asmy_game_instance_2)) 60.0))
  (set `self.DefaultScale` (`SceneComponent.K2_GetComponentScale` (`self.Bomb`))))

(event `self.ReceiveTick`
  (params (DeltaSeconds :type "Float (single-precision)"))
  (bind _ureversetimecomponent (`self.UReverseTimeComponent`))
  (bind _reversing (`/Game/Reverse/UReverseTimeComponent.Reversing` _ureversetimecomponent))
  (`|ExecutionSequence`
    (:`then_0`
      (set `self.Delta Seconds` DeltaSeconds)
      (set `self.DeltaTime` (+ (`KismetMathLibrary.SelectFloat` (* -1 (* (`self.Delta Seconds`) (`MyGameInstance.ReverseSpeed` (`self.As My Game Instance`)))) (`self.Delta Seconds`) (`/Game/ThirdPersonBP/Blueprints/Skill/PlayerSkillManager.IsReverse` (`/Game/ThirdPersonBP/Blueprints/ThirdPersonCharacter.PlayerSkillManager` (`self.As Third Person Character`)))) (`self.DeltaTime`)))
      (if (`/Game/Reverse/UReverseTimeComponent.Reversing` (`self.UReverseTimeComponent`))
        (`|ExecutionSequence`
          (:`then_0`
            (if (not (`self.IsWaitingTime`))
              (set `self.IsWaitingTime` true)))
          (:`then_1`
            ;[0.2257 0.6055 1] 爆発準備処理
            (if (`self.IsFuseTime`)
              (`self.Rev_Update Fuse`)))
          (:`then_2`
            ;[0.2257 0.6055 1] 爆発処理
            (if (`self.IsExplodeTime`)
              (`self.Rev_UpdateExplode`)))
          (:`then_3`
            (if (`self.IsEndProcess`)
              (bind _output_get (set `self.DeathTime` (- (`self.DeathTime`) (`self.Delta Seconds`))))
              (if (<= _output_get 0.0)
                (set `self.IsExplodeTime` true)
                (set `self.IsEndProcess` false)
                (set `self.DeathTime` 0.0)))))
        (else
          (`|ExecutionSequence`
            (:`then_0`
              ;[0.2257 0.6055 1] 待機モーション
              (if (`self.IsWaitingTime`)
                (`self.UpdateWaiting`)))
            (:`then_1`
              ;[0.2257 0.6055 1] 爆発準備処理
              (if (`self.IsFuseTime`)
                (`self.Update Fuse`)))
            (:`then_2`
              ;[0.2257 0.6055 1] 爆発処理
              (if (`self.IsExplodeTime`)
                (`self.UpdateExplode`)))
            (:`then_3`
              (if (`self.IsEndProcess`)
                (if (not (< (`self.DeltaTime`) 4.5))
                  (set `self.DeathTime` (+ (`self.DeathTime`) (`self.Delta Seconds`)))
                  (if (>= (`self.DeathTime`) (`self.DeathWaitTime`))
                    (`self.K2_DestroyActor`)
                    (else
                      (`PrimitiveComponent.SetCollisionEnabled` (`self.Sphere`) "NoCollision"))))))))))
    (:`then_1`
      (`/Engine/EditorBlueprintResources/StandardMacros.IsValid` self
        (:`Is Valid`
          (bind _output_get_2 (set `self.ActSurvivalTime` (+ (`self.ActSurvivalTime`) (`KismetMathLibrary.SelectFloat` (* (* DeltaSeconds (`/Game/Reverse/UReverseTimeComponent.ReverseSpeed` _ureversetimecomponent)) -1.0) DeltaSeconds _reversing))))
          (if (and (<= _output_get_2 0.1) _reversing)
            (`self.K2_DestroyActor`)))))))

(event `self.Sphere.OnComponentBeginOverlap`
  (params (OverlappedComponent :type "PrimitiveComponent Object Reference") (OtherActor :type "Actor Object Reference") (OtherComp :type "PrimitiveComponent Object Reference") (OtherBodyIndex :type Integer) (bFromSweep :type Boolean) (SweepResult :type "HitResult Structure (by ref)"))
  (bind _returnvalue (`self.ActorHasTag` OtherActor "Enemy"))
  (bind _returnvalue_2 (* (`KismetMathLibrary.Normal` (- (`self.K2_GetActorLocation`) (`self.K2_GetActorLocation` (`GameplayStatics.GetPlayerPawn` 0)))) (`self.BlowForce`)))
  ;[1 0.3838 0.8924] 剣か銃弾に当たったら
  (for _array_element (`ActorComponent.ComponentTags` OtherComp)
    _)
  (if (`self.IsWaitingTime`)
    ;[1 1 1] 初回ヒットで物理判定付与
    (`PrimitiveComponent.SetSimulatePhysics` (`self.Bomb`) true)
    ;[1 1 1] コリジョン削除
    (`PrimitiveComponent.SetCollisionEnabled` (`self.Sphere`) "NoCollision")
    ;[1 1 1] あたった方向に飛ばす
    (`PrimitiveComponent.AddImpulse` (`self.Bomb`) (`KismetMathLibrary.SelectVector` (* _returnvalue_2 4.6) _returnvalue_2 (== _array_element "PlayerSword")) "None" true)
    ;[1 1 1] 爆発処理開始
    (`self.StartFuse`)
    (set `self.DeltaTime` 0.0)
    (`GameplayStatics.PlaySoundAtLocation` "/Game/Sounds/SE/PlayerSE/SE_HitingSelf_Cue.SE_HitingSelf_Cue" (`self.K2_GetActorLocation`) (struct) 0.6 1.7 0.0 null null null)
    (elif (or (`self.ActorHasTag` OtherActor "Player") _returnvalue)
      (if (<= (`KismetArrayLibrary.Array_Find` (`self.hitobj`) OtherActor) -1)
        (`KismetArrayLibrary.Array_Add` (`self.hitobj`) OtherActor)
        (`GameplayStatics.ApplyDamage` OtherActor (`KismetMathLibrary.SelectFloat` (`self.EnemyDamage`) (`self.PlayerDamage`) _returnvalue) null self)))))

(fn `Rev_Update Fuse`
  (bind _p_smoke (`self.p_smoke`))
  ;[1 1 1] 4秒経過したら煙消して次へ
  (if (<= (`self.DeltaTime`) 0.0)
    (set `self.IsFuseTime` false)
    (set `self.IsExplodeTime` false)
    (`PrimitiveComponent.SetSimulatePhysics` (`self.Bomb`) false)
    (`PrimitiveComponent.SetCollisionEnabled` (`self.Sphere`) "QueryOnly")
    (`/Engine/EditorBlueprintResources/StandardMacros.IsValid` _p_smoke
      (:`Is Valid`
        (`ActorComponent.K2_DestroyComponent` _p_smoke)))))

(fn `Rev_UpdateExplode`
  (bind _p_smoke (`self.p_smoke`))
  (if (>= (`self.DeltaTime`) 4.0)
    (`SceneComponent.SetWorldScale3D` (`self.Bomb`) (- (`self.GetActorScale3D`) 0.05))
    (`SceneComponent.SetVisibility` (`self.Bomb`) true false)
    (else
      (`PrimitiveComponent.SetCollisionResponseToChannel` (`self.Bomb`) "ECC_Pawn" "ECR_Ignore")
      (`PrimitiveComponent.SetCollisionResponseToChannel` (`self.Bomb`) "ECC_GameTraceChannel2" "ECR_Ignore")
      (set `self.IsExplodeTime` false)
      (set `self.IsFuseTime` true)
      (`SceneComponent.SetVisibility` (`self.Bomb`) true false)
      (`SphereComponent.SetSphereRadius` (`self.Sphere`) 32.0 true)
      (`SceneComponent.SetWorldScale3D` (`self.Bomb`) (`self.DefaultScale`))
      (`/Engine/EditorBlueprintResources/StandardMacros.IsValid` _p_smoke
        (:`Is Valid`
          (`ActorComponent.K2_DestroyComponent` _p_smoke))))))

(fn `StartFuse`
  ;[0.1866 0.6345 1] 煙出してフューズへ移行する
  (bind _returnvalue (`GameplayStatics.SpawnEmitterAttached` "/Game/StarterContent/Particles/P_Smoke.P_Smoke" (`self.Bomb`) "None" (0.0 0.0 0.0) (struct) (5.0 5.0 5.0)))
  (bind _output_get (set `self.p_smoke` _returnvalue))
  (`SceneComponent.SetAbsolute` _output_get false true false)
  (set `self.IsWaitingTime` false)
  (set `self.IsFuseTime` true))

(fn `Update Fuse`
  (bind _p_smoke (`self.p_smoke`))
  ;[1 1 1] 4秒経過したら煙消して次へ
  (if (>= (`self.DeltaTime`) 4.0)
    (set `self.IsFuseTime` false)
    (set `self.IsExplodeTime` true)
    (`PrimitiveComponent.SetCollisionResponseToChannel` (`self.Bomb`) "ECC_WorldDynamic" "ECR_Block")
    (`PrimitiveComponent.SetCollisionResponseToChannel` (`self.Bomb`) "ECC_GameTraceChannel1" "ECR_Block")
    (`/Engine/EditorBlueprintResources/StandardMacros.IsValid` _p_smoke
      (:`Is Valid`
        (`ActorComponent.K2_DestroyComponent` _p_smoke)))))

(fn `UpdateExplode`
  (if (< (`self.DeltaTime`) 4.2)
    (`SceneComponent.SetWorldScale3D` (`self.Bomb`) (+ (`self.GetActorScale3D`) 0.05))
    (else
      ;[0.7699 0.4283 1] 爆発処理して終了
      (`GameplayStatics.SpawnEmitterAtLocation` "/Game/StarterContent/Particles/P_Explosion.P_Explosion" (`SceneComponent.GetSocketLocation` (`self.Bomb`) "None") (struct) (4.0 4.0 4.0))
      (set `self.IsExplodeTime` false)
      (set `self.IsEndProcess` true)
      (`PrimitiveComponent.SetCollisionEnabled` (`self.Sphere`) "QueryOnly")
      (`SphereComponent.SetSphereRadius` (`self.Sphere`) 150.0 true)
      (`SceneComponent.SetVisibility` (`self.Bomb`) false false)
      (`GameplayStatics.PlaySoundAtLocation` "/Game/StarterContent/Audio/Explosion_Cue.Explosion_Cue" (`SceneComponent.GetSocketLocation` (`self.Bomb`) "None") (struct) 1.0 1.0 0.0 null null null))))

(fn `UpdateWaiting`
  (`self.K2_AddActorLocalRotation` (`KismetMathLibrary.MakeRotator` 0.0 0.0 (* (`self.Delta Seconds`) 100.0))))

(fn `UserConstructionScript`)