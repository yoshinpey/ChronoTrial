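; Bomb spawner actor that periodically spawns BP_Bomb at a random free point among spawners sharing its TagSpawner, with an optional spawn on BeginPlay.
; The first spawner per tag to begin play becomes leader and gathers the group.
; While enabled, the leader's Tick runs the interval timer, rewinding it without spawning during player time reversal.
; Spawn skips points with a bomb within a small radius.
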(event `self.ReceiveBeginPlay`
  (bind _asthird_person_character (cast `/Game/ThirdPersonBP/Blueprints/ThirdPersonCharacter` (`GameplayStatics.GetPlayerPawn` 0))
    (:`then`
      (set `self.Player` _asthird_person_character)
      (bind _asmy_game_instance (cast `MyGameInstance` (`GameplayStatics.GetGameInstance`))
        (:`then`
          (set `self.ReverseSpeed` (`MyGameInstance.ReverseSpeed` _asmy_game_instance))
          (if (`self.FirstSpawn`)
            (`|SpawnActorFromClass` "/Game/ExplodeObject/BP_Bomb.BP_Bomb_C" (`KismetMathLibrary.MakeTransform` (`self.K2_GetActorLocation`)) "Undefined" "OverrideRootScale" null null))
          ;[1 1 1] Readerを探し・所属Ｂｏｍｂたちの追加
          (set `self.RandSelectInGame` false)
          (bind _outactors (`GameplayStatics.GetAllActorsOfClass` "BP_BombSpawner_C"))
          (for _array_element _outactors
            (if (!= _array_element self)
              (if (== (`/Game/ExplodeObject/BP_BombSpawner.TagSpawner` _array_element) (`self.TagSpawner`))
                (if (`/Game/ExplodeObject/BP_BombSpawner.RandSelectConstructEnd` _array_element)
                  (set `self.RandSelectInGame` true)
                  (break)))))
          (set `self.RandSelectConstructEnd` true)
          (if (not (`self.RandSelectInGame`))
            (set `self.ReaderRandSelect` true)
            (bind _outactors_2 (`GameplayStatics.GetAllActorsOfClass` "BP_BombSpawner_C"))
            (for _array_element_2 _outactors_2
              (if (== (`/Game/ExplodeObject/BP_BombSpawner.TagSpawner` _array_element_2) (`self.TagSpawner`))
                (`KismetArrayLibrary.Array_Add` (`self.RandSelects`) _array_element_2)))))
        (:`CastFailed`
          (`KismetSystemLibrary.PrintString` "BombSpawner_CastError"))))
    (:`CastFailed`
      (`KismetSystemLibrary.PrintString` "BombSpawner_CastError"))))

(event `self.ReceiveTick`
  (params (DeltaSeconds :type "Float (single-precision)"))
  (`|ExecutionSequence`
    (:`then_0`
      (if (and (`self.ReaderRandSelect`) (`self.IsSpawnerEnable`))
        (if (`/Game/ThirdPersonBP/Blueprints/ThirdPersonCharacter.IsReverse` (`self.Player`))
          ;[1 1 1] Reverse
          (if (`/Game/ThirdPersonBP/Blueprints/ThirdPersonCharacter.IsReverse` (`self.Player`))
            (set `self.ElapsedTime` (- (`self.ElapsedTime`) (* (`self.ReverseSpeed`) DeltaSeconds)))
            (if (< (`self.ElapsedTime`) 0.0)
              (set `self.ElapsedTime` (`self.IntervalTime`))))
          (else
            ;[1 1 1] 通常スポーン処理
            (bind _output_get (set `self.ElapsedTime` (+ DeltaSeconds (`self.ElapsedTime`))))
            (if (> _output_get (`self.IntervalTime`))
              (`self.Spawn`)
              (set `self.ElapsedTime` (- (`self.ElapsedTime`) (`self.IntervalTime`))))))))))

(fn `Spawn`
  (locals (SubRandSelect :type "Array of /Game/ExplodeObject/BP_BombSpawner Object Reference") (AllBombLeng :type Boolean))
  (bind _subrandselect (`local.SubRandSelect`))
  (bind _returnvalue (`KismetArrayLibrary.Array_Length` _subrandselect))
  (`KismetArrayLibrary.Array_Clear` (`local.SubRandSelect`))
  (for _array_element (`self.RandSelects`)
    (set `local.AllBombLeng` true)
    (bind _outactors (`GameplayStatics.GetAllActorsOfClass` "/Game/ExplodeObject/BP_Bomb.BP_Bomb_C"))
    (for _array_element_2 _outactors
      (if (<= (`KismetMathLibrary.VSize` (- (`self.K2_GetActorLocation` _array_element_2) (`self.K2_GetActorLocation` _array_element))) 10.0)
        (set `local.AllBombLeng` false)
        (break)))
    (if (`local.AllBombLeng`)
      (`KismetArrayLibrary.Array_AddUnique` (`local.SubRandSelect`) _array_element)))
  (if (>= _returnvalue 1)
    (`|SpawnActorFromClass` "/Game/ExplodeObject/BP_Bomb.BP_Bomb_C" (`KismetMathLibrary.MakeTransform` (`self.K2_GetActorLocation` (`|GetArrayItem` _subrandselect (`KismetMathLibrary.RandomInteger` _returnvalue)))) "Undefined" "OverrideRootScale" null null)))

(fn `UserConstructionScript`)